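; BP_fruit is a hittable fruit that swaps its intact mesh for a breakable version when hit.
; SMSphereDm starts hidden at BeginPlay while the Fruit component represents the whole fruit.
; onHit hides Fruit, then reveals SMSphereDm and enables its physics.
; It then applies a small radial damage at the Container's location, apparently to fracture the revealed mesh.
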(event `self.ReceiveBeginPlay`
  (`SceneComponent.SetVisibility` (`self.SM_sphere_dm`) false false))

(event `onHit`
  (bind _sm_sphere_dm (`self.SM_sphere_dm`))
  (`SceneComponent.SetVisibility` (`self.fruit`) false false)
  (`SceneComponent.SetVisibility` _sm_sphere_dm true false)
  (`PrimitiveComponent.SetSimulatePhysics` _sm_sphere_dm true)
  (`GameplayStatics.ApplyRadialDamage` :`BaseDamage` 1.0 :`Origin` (`SceneComponent.K2_GetComponentLocation` (`self.Container`)) :`DamageRadius` 1.0 :`DamageCauser` null :`InstigatedByController` null))

(fn `UserConstructionScript`)